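; StoneMove is a 2D stone object that repeatedly moves between two relative positions and changes its face, using SMB3 object sprites.
; After a short delay on BeginPlay, a timeline lerps the PaperSprite's location without sweep, then restarts after a pause each time it finishes.
; Each timeline update also picks one of two sprites, switching when the timeline value crosses a threshold near its upper end.
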(event Custom|DropDown
  (bind _speed (Timeline|TimelineAnimation PlayFromStart)
    (:Update
      (Utilities|FlowControl|Sequence
        (:then_0
          (Transformation|SetRelativeLocation (Variables|Default|GetPaperSprite) (Math|Vector|Lerp(Vector) (Variables|Default|GetA) (Variables|Default|GetB) _speed) false false))
        (:then_1
          (CallFunction|ChangeFace))))
    (:Finished
      (Utilities|FlowControl|Delay 1.0)
      (CallFunction|DropDown))))

(event Custom|ChangeFace
  (if (>= (stale Custom|DropDown _speed) 0.8)
    (Rendering|Components|Sprite|SetSprite (Variables|Default|GetPaperSprite) "/Game/Asset2_Mario/SMB3_Objects_Sprite_388.SMB3_Objects_Sprite_388")
    (else
      (Rendering|Components|Sprite|SetSprite (Variables|Default|GetPaperSprite) "/Game/Asset2_Mario/SMB3_Objects_Sprite_371.SMB3_Objects_Sprite_371"))))

(event EventBeginPlay
  (Utilities|FlowControl|Delay 1.0)
  (CallFunction|DropDown))

(fn ConstructionScript)