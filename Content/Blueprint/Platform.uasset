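; One-way platform actor for MyCharacter that toggles the collision of its RenderComponent, tracked by a Status flag.
; Entering UpperBox turns collision on, and leaving it turns collision off after a short delay.
; Pressing C turns collision off at once to allow dropping through.
; Overlapping LowerBox enables the actor's input for player 0, which is never disabled again here.
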(event OnComponentBeginOverlap(UpperBox)
  (params (OverlappedComponent :type Primitive%20Component%20Object%20Reference) (OtherActor :type Actor%20Object%20Reference) (OtherComp :type Primitive%20Component%20Object%20Reference) (OtherBodyIndex :type Integer) (bFromSweep :type Boolean) (SweepResult :type Hit%20Result%20Structure%20%28by%20ref%29))
  (Utilities|Casting|CastToMyCharacter OtherActor)
  (if (not (Variables|Default|GetStatus))
    (Collision|SetCollisionEnabled (Variables|Default|GetRenderComponent) "QueryAndPhysics")
    (Variables|Default|SetStatus true)))

(event OnComponentBeginOverlap(LowerBox)
  (params (OverlappedComponent :type Primitive%20Component%20Object%20Reference) (OtherActor :type Actor%20Object%20Reference) (OtherComp :type Primitive%20Component%20Object%20Reference) (OtherBodyIndex :type Integer) (bFromSweep :type Boolean) (SweepResult :type Hit%20Result%20Structure%20%28by%20ref%29))
  (Utilities|Casting|CastToMyCharacter OtherActor)
  (Input|EnableInput (Game|GetPlayerController 0)))

(event OnComponentEndOverlap(UpperBox)
  (params (OverlappedComponent :type Primitive%20Component%20Object%20Reference) (OtherActor :type Actor%20Object%20Reference) (OtherComp :type Primitive%20Component%20Object%20Reference) (OtherBodyIndex :type Integer))
  (Utilities|Casting|CastToMyCharacter OtherActor)
  (if (Variables|Default|GetStatus)
    (Utilities|FlowControl|Delay 0.5)
    (Collision|SetCollisionEnabled (Variables|Default|GetRenderComponent) "NoCollision")
    (Variables|Default|SetStatus false)))

(event EventBeginPlay)

(event Input|KeyboardEvents|C
  (params (Key :type Key%20Structure :default "None"))
  (:Pressed
    (if (Variables|Default|GetStatus)
      (Collision|SetCollisionEnabled (Variables|Default|GetRenderComponent) "NoCollision")
      (Variables|Default|SetStatus false))))

(fn ConstructionScript)