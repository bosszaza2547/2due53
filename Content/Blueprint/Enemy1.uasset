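; Enemy1 is a Paper2D patrolling enemy that walks forward and dies when hit by an actor tagged "Player Bullet", destroying both.
; Each Tick drives movement, picks the walk or idle flipbook from velocity, and records horizontal direction in IsMovingRight.
; Line traces from two detectors then flip its rotation when the floor ends or a wall blocks it.
; The wall trace always points along world +X, regardless of facing.
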(event OnComponentBeginOverlap(CapsuleComponent)
  (params (OverlappedComponent :type Primitive%20Component%20Object%20Reference) (OtherActor :type Actor%20Object%20Reference) (OtherComp :type Primitive%20Component%20Object%20Reference) (OtherBodyIndex :type Integer) (bFromSweep :type Boolean) (SweepResult :type Hit%20Result%20Structure%20%28by%20ref%29))
  ;[1 1 1] Player Bullet Check
  (if (Actor|ActorHasTag OtherActor "Player Bullet")
    (Actor|DestroyActor OtherActor)
    (Actor|DestroyActor)))

(event Custom|CheckDirection
  (if (> (.x (Transformation|GetVelocity)) 0.0)
    (Variables|Default|SetIsMovingRight true)
    (elif (< (.x (Transformation|GetVelocity)) 0.0)
      (Variables|Default|SetIsMovingRight false))))

(event Custom|MoveForward
  (Pawn|Input|AddMovementInput (Transformation|GetActorForwardVector) 1.0 false))

(event Custom|UpdateAnimation
  (Sprite|SetFlipbook (Variables|Default|GetPaperFlipbook) (select (> (Math|Vector|VectorLength (Transformation|GetVelocity)) 0.0) "/Game/Asset3_Flipbooks/EnemyWalk.EnemyWalk" "/Game/Asset3_Flipbooks/EnemyIdle.EnemyIdle")))

(event Custom|TurnChar
  (Transformation|SetActorRotation (Math|Rotator|CombineRotators (Transformation|GetActorRotation) "0.000000,180.000000,0.000000")))

(event Custom|WallCheck
  (bind _walldetector (Variables|Default|GetWallDetector))
  (bind _outhit (Collision|LineTraceByChannel (Transformation|GetWorldLocation _walldetector) (+ (Transformation|GetWorldLocation _walldetector) "20.000000,0.000000,0.000000") "TraceTypeQuery1" false 0 "None"))
  (if (.bBlockingHit (Collision|BreakHitResult _outhit))
    (CallFunction|TurnChar)))

(event Custom|EdgeCheck
  (bind _edgedetector (Variables|Default|GetEdgeDetector))
  (bind _outhit (Collision|LineTraceByChannel (Transformation|GetWorldLocation _edgedetector) (- (Transformation|GetWorldLocation _edgedetector) "0.000000,0.000000,200.000000") "TraceTypeQuery1" false 0 "None"))
  (if (not (.bBlockingHit (Collision|BreakHitResult _outhit)))
    (CallFunction|TurnChar)))

(event EventTick
  (params (DeltaSeconds :type Float%20%28single-precision%29))
  (Utilities|FlowControl|Sequence
    (:then_0
      (CallFunction|MoveForward)
      (CallFunction|UpdateAnimation)
      (CallFunction|CheckDirection))
    (:then_1
      (CallFunction|EdgeCheck)
      (CallFunction|WallCheck))))

(fn ConstructionScript)